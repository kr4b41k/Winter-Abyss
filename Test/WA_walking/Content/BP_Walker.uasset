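; BP_Walker is a controllable Walker with a mesh and camera that turns its view with mouse input.
; MouseMoveX and MouseMoveY feed controller yaw and pitch, and each yaw input also prints the CosMeshCam result as debug output.
; CosMeshCam flattens the mesh and camera forward vectors to 2D and divides their product by their lengths, as a horizontal angle-cosine measure.
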(event `InputAxis|MouseMoveX`
  (params (AxisValue :type "Float (single-precision)"))
  (`self.AddControllerYawInput` AxisValue)
  (`KismetSystemLibrary.PrintString` (`KismetStringLibrary.Conv_Vector2dToString` (`self.CosMeshCam`))))

(event `InputAxis|MouseMoveY`
  (params (AxisValue :type "Float (single-precision)"))
  (`self.AddControllerPitchInput` AxisValue))

(fn `CosMeshCam`
  (returns (ReturnValue :type "Vector2D Structure"))
  (bind _returnvalue (`KismetMathLibrary.Conv_VectorToVector2D` (`SceneComponent.GetForwardVector` (`self.Camera`))))
  (bind _returnvalue_2 (`KismetMathLibrary.Conv_VectorToVector2D` (`SceneComponent.GetForwardVector` (`self.Mesh`))))
  (return (/ (* _returnvalue_2 _returnvalue) (* (`KismetMathLibrary.VSize2D` _returnvalue_2) (`KismetMathLibrary.VSize2D` _returnvalue)))))

(fn `UserConstructionScript`)